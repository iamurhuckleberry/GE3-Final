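; BP_Button2 is a pressure button that changes color and rotates the level's BP_Door through capsule overlaps.
; A BP_Box entering turns the button green and plays a timeline driving the door's yaw.
; A BP_ThirdPersonCharacter leaving, rather than the box, turns it red and plays a second yaw timeline.
; Each event creates a dynamic material and finds the door with GetActorOfClass; a character cast for entering is left unconnected.
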(event OnComponentBeginOverlap(Capsule)
  (params (OverlappedComponent :type Primitive%20Component%20Object%20Reference) (OtherActor :type Actor%20Object%20Reference) (OtherComp :type Primitive%20Component%20Object%20Reference) (OtherBodyIndex :type Integer) (bFromSweep :type Boolean) (SweepResult :type Hit%20Result%20Structure%20%28by%20ref%29))
  (Utilities|Casting|CastToBP_Box OtherActor)
  (bind _returnvalue (Rendering|Material|CreateDynamicMaterialInstance (Variables|Default|Getbutton) 0 "/Game/MyProps/Button_Color.Button_Color" "None" :!class /Script/Engine.PrimitiveComponent))
  (Rendering|Material|SetVectorParameterValue _returnvalue "Color01" (Utilities|Struct|MakeLinearColor 0.0 255.0 0.0 0.0) :!class /Script/Engine.MaterialInstanceDynamic)
  (bind _returnvalue_2 (Actor|GetActorOfClass "/Game/My_BP/BP_Door.BP_Door_C"))
  (bind _output_get (Variables|Default|SetDoorRotate _returnvalue_2))
  (bind _新建轨道_0 (Timeline|时间轴_0 Play)
    (:Update
      (Transformation|SetRelativeRotation (Variables|/Script/Engine.Actor|GetRootComponent _output_get) (Math|Rotator|MakeRotator 0.0 0.0 _新建轨道_0) false false))))

(event OnComponentEndOverlap(Capsule)
  (params (OverlappedComponent :type Primitive%20Component%20Object%20Reference) (OtherActor :type Actor%20Object%20Reference) (OtherComp :type Primitive%20Component%20Object%20Reference) (OtherBodyIndex :type Integer))
  (Utilities|Casting|CastToBP_ThirdPersonCharacter OtherActor)
  (bind _returnvalue (Rendering|Material|CreateDynamicMaterialInstance (Variables|Default|Getbutton) 0 "/Game/MyProps/Button_Color.Button_Color" "None" :!class /Script/Engine.PrimitiveComponent))
  (Rendering|Material|SetVectorParameterValue _returnvalue "Color01" (Utilities|Struct|MakeLinearColor 255.0 0.0 0.0 0.0) :!class /Script/Engine.MaterialInstanceDynamic)
  (bind _returnvalue_2 (Actor|GetActorOfClass "/Game/My_BP/BP_Door.BP_Door_C"))
  (bind _output_get (Variables|Default|SetDoorRotate _returnvalue_2))
  (bind _新建轨道_0 (Timeline|时间轴_1 Play)
    (:Update
      (Transformation|SetRelativeRotation (Variables|/Script/Engine.Actor|GetRootComponent _output_get) (Math|Rotator|MakeRotator 0.0 0.0 _新建轨道_0) false false))))

(event EventBeginPlay
  (|CallParentFunction) ; 此节点被禁用，将不会被调用。\n从引脚连出引线来编译功能。
)

(event Collision|EventActorBeginOverlap
  (params (OtherActor :type Actor%20Object%20Reference))
  (|CallParentFunction OtherActor) ; 此节点被禁用，将不会被调用。\n从引脚连出引线来编译功能。
)

(event EventTick
  (params (DeltaSeconds :type Float%20%28single-precision%29))
  (|CallParentFunction DeltaSeconds) ; 此节点被禁用，将不会被调用。\n从引脚连出引线来编译功能。
)

(fn ConstructionScript
  (|CallParentFunction))