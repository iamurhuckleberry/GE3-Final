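; BP_Button_Firework is a trigger button that starts a firework show when the third-person character touches it.
; Its Capsule overlap event finds a BP_Firework actor in the level by class, stores it and activates its Niagara component.
; It then hides every DirectionalLight actor in game, with no logic to restore the lights or stop the effect.
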(event OnComponentBeginOverlap(Capsule)
  (params (OverlappedComponent :type Primitive%20Component%20Object%20Reference) (OtherActor :type Actor%20Object%20Reference) (OtherComp :type Primitive%20Component%20Object%20Reference) (OtherBodyIndex :type Integer) (bFromSweep :type Boolean) (SweepResult :type Hit%20Result%20Structure%20%28by%20ref%29))
  (Utilities|Casting|CastToBP_ThirdPersonCharacter OtherActor)
  (bind _returnvalue (Actor|GetActorOfClass "/Game/My_BP/BP_Firework.BP_Firework_C"))
  (bind _output_get (Variables|Default|SetFireWork _returnvalue))
  (Components|Activation|SetActive (Variables|/Game/My_BP/BP_Firework.BP_Firework_C|GetNiagara _output_get) true false)
  (bind _outactors (Actor|GetAllActorsOfClass "/Script/Engine.DirectionalLight"))
  (for _array_element _outactors
    (Rendering|SetActorHiddenInGame _array_element true)))

(event EventBeginPlay
  (|CallParentFunction) ; 此节点被禁用，将不会被调用。\n从引脚连出引线来编译功能。
)

(event Collision|EventActorBeginOverlap
  (params (OtherActor :type Actor%20Object%20Reference))
  (|CallParentFunction OtherActor) ; 此节点被禁用，将不会被调用。\n从引脚连出引线来编译功能。
)

(event EventTick
  (params (DeltaSeconds :type Float%20%28single-precision%29))
  (|CallParentFunction DeltaSeconds) ; 此节点被禁用，将不会被调用。\n从引脚连出引线来编译功能。
)

(fn ConstructionScript
  (|CallParentFunction))